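; Spear projectile actor that damages fish it hits or hands itself back to the player when it strikes anything else.
; Each tick it rotates to face along its velocity.
; A fish hit lowers that fish's health and tells the player character (FPSPlayerController) to despawn the spear.
; Any other hit calls SpawnSpear on that character, passing the impact location, mesh rotation and itself.
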(event Custom|HitGround
  (params (HitLocation :type Vector))
  ;[1 1 1] Hit Ground
  (bind _asfpsplayer_controller (Utilities|Casting|CastToFPSPlayerController (Game|GetPlayerCharacter 0)))
  (Default|SpawnSpear _asfpsplayer_controller (Math|Transform|MakeTransform HitLocation (Transformation|GetWorldRotation (Variables|Debug|GetStaticMeshComponent)) "1,1,1") self))

(event Custom|HitFish
  (params (Fish :type Fish%20BP%20Object%20Reference))
  ;[1 1 1] Hit Fish
  (bind _asfish_bp (Utilities|Casting|CastToFishBP Fish))
  (Default|ChangeFishHealthby _asfish_bp -1.0)
  (bind _asfpsplayer_controller (Utilities|Casting|CastToFPSPlayerController (Game|GetPlayerCharacter 0)))
  (Default|DespawnSpear _asfpsplayer_controller))

(event EventBeginPlay)

(event Collision|EventActorBeginOverlap
  (params (OtherActor :type Actor%20Object%20Reference)))

(event EventTick
  (params (DeltaSeconds :type Float%20%28single-precision%29))
  (bind _staticmeshcomponent (Variables|Debug|GetStaticMeshComponent))
  (bind _returnvalue (Transformation|GetWorldLocation _staticmeshcomponent))
  (Transformation|SetActorRotation (Math|Rotator|FindLookatRotation _returnvalue (+ _returnvalue (Transformation|GetVelocity)))))

(event Collision|EventHit
  (params (MyComp :type Primitive%20Component%20Object%20Reference) (Other :type Actor%20Object%20Reference) (OtherComp :type Primitive%20Component%20Object%20Reference) (bSelfMoved :type Boolean) (HitLocation :type Vector :default "0, 0, 0") (HitNormal :type Vector :default "0, 0, 0") (NormalImpulse :type Vector :default "0, 0, 0") (Hit :type Hit%20Result%20Structure%20%28by%20ref%29))
  (bind _asfish_bp (Utilities|Casting|CastToFishBP Other)
    (:then
      (CallFunction|HitFish _asfish_bp))
    (:CastFailed
      (CallFunction|HitGround HitLocation))))

(fn ConstructionScript)