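; Fish3 is an enemy fish that wanders, attacks the player with spit projectiles, and can be killed.
; Tick checks whether the player is within range, then after random delays either faces and chases them while spawning Projectile_2, or moves to a random reachable point.
; Health changes flash a blood effect; at zero the fish passes that last change value to the player's money and destroys itself.
; TailSlap only nudges pitch and is not called here.
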(event Custom|ChangeFishHealthBy
  (params (Value :type Float%20%28single-precision%29))
  ;[1 1 1] Health
  (bind _output_get (Variables|Default|SetHealth (+ Value (Variables|Default|GetHealth))))
  (Components|Activation|Activate (Variables|Default|Getm_bloodimpact) false)
  (Utilities|FlowControl|Delay 0.2)
  (Components|Activation|Deactivate (Variables|Default|Getm_bloodimpact))
  (if (<= _output_get 0.0)
    (bind _asfpsplayer_controller (Utilities|Casting|CastToFPSPlayerController (Game|GetPlayerCharacter 0)))
    (Default|ChangePlayerMoneyby _asfpsplayer_controller (Variables|Default|GetValue))
    (Actor|DestroyActor)))

(event Custom|Check%20Distance%20From%20Player
  (if (<= (Transformation|GetDistanceTo (Variables|Default|GetPlayer)) 4e+03)
    (Variables|Default|SetisAttackingPlayer true)
    (else
      (Variables|Default|SetisAttackingPlayer false))))

(event Custom|Spit%20Attack
  ;[1 1 1] Spit Attack
  (Utilities|FlowControl|Delay (Math|Random|RandomFloatinRange 0.5 3.0))
  (Game|SpawnActorfromClass "/Game/Blueprints/Projectile_2.Projectile_2_C" (Math|Transform|MakeTransform (Transformation|GetWorldLocation (Variables|Default|GetProjectileRef)) (Transformation|GetWorldRotation (Variables|Collision|GetCapsuleComponent))) "Undefined" 0 0))

(event Custom|Tail%20Slap
  ;[1 1 1] Tail Slap
  (Utilities|FlowControl|Delay (Math|Random|RandomFloatinRange 0.5 3.0))
  (Transformation|AddActorLocalRotation (Math|Rotator|MakeRotator 0.0 1.0 0.0) false false))

(event EventBeginPlay
  (bind _asfpsplayer_controller (Utilities|Casting|CastToFPSPlayerController (Game|GetPlayerCharacter 0)))
  (Variables|Default|SetPlayer _asfpsplayer_controller))

(event EventTick
  (params (DeltaSeconds :type Float%20%28single-precision%29))
  (CallFunction|CheckDistancefromPlayer)
  (Utilities|FlowControl|Delay (Math|Random|RandomFloatinRange 1.0 5.0))
  (if (Variables|Default|GetisAttackingPlayer)
    (Transformation|SetActorRotation (Math|Rotator|FindLookatRotation (Transformation|GetActorLocation) (Transformation|GetActorLocation (Variables|Default|GetPlayer))))
    (AI|AIMoveTo self "0, 0, 0" (Variables|Default|GetPlayer) 1.0 false
      (:then
        (CallFunction|SpitAttack)))
    (else
      (Variables|Default|SetIsMoving true)
      (AI|AIMoveTo self (.RandomLocation (AI|Navigation|GetRandomReachablePointinRadius (Transformation|GetActorLocation) 3e+03 0 0)) 0 1.0 false
        (:OnSuccess
          _)
        (:OnFail
          _))
      (Variables|Default|SetIsMoving false))))

(fn ConstructionScript)