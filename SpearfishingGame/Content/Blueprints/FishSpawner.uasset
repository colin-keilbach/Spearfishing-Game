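; FishSpawner is a Blueprint that repeatedly spawns AI fish at its scene root's location.
; Tick feeds a Delay, which acts as a timer that triggers a spawn roughly every five seconds.
; Two nested random rolls weight the choice between FishBP as the most common, Fish2 slightly less common and Fish3 as the rare one.
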(event EventTick
  (params (DeltaSeconds :type Float%20%28single-precision%29))
  (bind _returnvalue (Math|Random|RandomFloatinRange 0.0 1e+02))
  (bind _defaultsceneroot (Variables|Default|GetDefaultSceneRoot))
  (bind _returnvalue_2 (Transformation|GetWorldLocation _defaultsceneroot))
  (Utilities|FlowControl|Delay 5.0)
  (if (<= _returnvalue 5e+01)
    (AI|SpawnAIFromClass "/Game/Blueprints/FishBP.FishBP_C" 0 _returnvalue_2 "0, 0, 0" false 0)
    (elif (<= _returnvalue 9e+01)
      (AI|SpawnAIFromClass "/Game/Blueprints/Fish2.Fish2_C" 0 _returnvalue_2 "0, 0, 0" false 0)
      (else
        (AI|SpawnAIFromClass "/Game/Blueprints/Fish3.Fish3_C" 0 _returnvalue_2 "0, 0, 0" false 0)))))

(fn ConstructionScript)