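; BP_Projectile is a projectile actor that damages a player on impact and removes itself.
; Its Hit event casts the hit actor to FPSPlayerController; on success, it passes the Damage variable to ChangePlayerHealthBy and destroys the projectile.
; Any other hit goes to HitGround, which only destroys the projectile.
; BeginPlay, overlap, Tick and the construction script hold no logic.
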(event Custom|Hit%20Player
  (params (Player :type FPS%20Player%20Controller%20Object%20Reference))
  ;[1 0 0] Damage Player
  (Default|ChangePlayerHealthby Player (Variables|Default|GetDamage))
  (Actor|DestroyActor self))

(event Custom|Hit%20Ground
  ;[0.3279 1 0.183] Collides with Ground
  (Actor|DestroyActor self))

(event EventBeginPlay)

(event Collision|EventActorBeginOverlap
  (params (OtherActor :type Actor%20Object%20Reference)))

(event EventTick
  (params (DeltaSeconds :type Float%20%28single-precision%29)))

(event Collision|EventHit
  (params (MyComp :type Primitive%20Component%20Object%20Reference) (Other :type Actor%20Object%20Reference) (OtherComp :type Primitive%20Component%20Object%20Reference) (bSelfMoved :type Boolean) (HitLocation :type Vector :default "0, 0, 0") (HitNormal :type Vector :default "0, 0, 0") (NormalImpulse :type Vector :default "0, 0, 0") (Hit :type Hit%20Result%20Structure%20%28by%20ref%29))
  (bind _asfpsplayer_controller (Utilities|Casting|CastToFPSPlayerController Other)
    (:then
      (CallFunction|HitPlayer _asfpsplayer_controller))
    (:CastFailed
      (CallFunction|HitGround))))

(fn ConstructionScript)