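; First-person player character, despite the controller name, with movement, a spear grapple, health and money.
; Tick handles buffered jumps for bunny hopping, low-braking crouch slides that lock move input, and the grapple pull.
; A thrown projectile becomes a spear object via SpawnSpear, adding velocity toward it and along camera forward until returned, with a Niagara rope tracking it.
; Air strafes add sideways velocity, and zero health quits the game.
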(event Custom|SpawnSpear
  (params (Transform :type Transform) (Spear :type Spear%20Projectile%20Object%20Reference))
  ;[0.227 1 0.1517] Spear has collided with ground
  (if (Utilities|IsValid Spear)
    (Actor|DestroyActor Spear)
    (bind _returnvalue (Game|SpawnActorfromClass "/Game/Blueprints/SpearObject.SpearObject_C" Transform "Undefined" 0 0))
    (bind _output_get (Variables|Default|SetSpearObject _returnvalue))
    (Class|NiagaraComponent|SetNiagaraVariableVec3 (Variables|Default|GetRope) "EndPosition" (Transformation|GetActorLocation _output_get))))

(event Custom|ChangePlayerHealthBy
  (params (Amount :type Float%20%28single-precision%29))
  ;[1 0.2188 0.2188] Player Health
  (bind _output_get (Variables|Default|SetPlayerHealth (+ Amount (Variables|Default|GetPlayerHealth))))
  (if (<= _output_get 0.0)
    (Game|QuitGame 0 "Quit" false)))

(event Custom|UpdateRope
  (params (Location :type Vector))
  (Class|NiagaraComponent|SetNiagaraVariableVec3 (Variables|Default|GetRope) "EndPosition" Location))

(event Custom|ChangePlayerMoneyBy
  (params (Amount :type Float%20%28single-precision%29))
  ;[1 0.2188 0.2188] Player Money
  (Variables|Default|SetMoney (+ Amount (Variables|Default|GetMoney))))

(event Custom|DespawnSpear
  (bind _spearobject (Variables|Default|GetSpearObject))
  ;[0.227 1 0.1517] Pull Spear
  (if (Variables|Default|GetSpearThrown)
    (if (Utilities|IsValid _spearobject)
      (Actor|DestroyActor _spearobject)
      (else
        (Actor|DestroyActor (Variables|Default|GetSpearProjectile))))
    (Variables|Default|SetSpearThrown false)
    (Class|NiagaraComponent|SetNiagaraVariableVec3 (Variables|Default|GetRope) "EndPosition" "10.000000, 0, 0")))

(event EventTick
  (params (DeltaSeconds :type Float%20%28single-precision%29))
  (bind _charactermovement (Variables|Character|GetCharacterMovement))
  (bind _charactermovement_2 (Variables|Character|GetCharacterMovement))
  (bind _charactermovement_3 (Variables|Character|GetCharacterMovement))
  (bind _returnvalue (AI|Components|NavMovement|IsMovingonGround _charactermovement_3))
  ;[1 0.9448 0.3267] Jump (Jump Buffer for bunny hopping)
  (bind _output_get (Variables|Default|SetJumpBuffer (- (stale Input|ActionEvents|InputActionJump _output_get) DeltaSeconds)))
  (if (and (>= _output_get 0.0) (AI|Components|NavMovement|IsMovingonGround (Variables|Character|GetCharacterMovement)))
    (Character|Jump))
  ;[1 0.9448 0.3267] Sliding
  (if (and (Variables|Default|GetCrouching) (> (Math|Vector|VectorLength (Variables|/Script/Engine.MovementComponent|GetVelocity _charactermovement_3)) 3e+02))
    (bind _output_get_2 (Variables|/Script/Engine.CharacterMovementComponent|SetBrakingDecelerationWalking _charactermovement 0.05))
    (Variables|/Script/Engine.CharacterMovementComponent|SetBrakingFrictionFactor _charactermovement _output_get_2)
    (if _returnvalue
      (Variables|Default|SetSliding true :!label _label)
      (else
        (Variables|Default|SetSliding false :!label _label_2)))
    (else
      (bind _output_get_3 (Variables|/Script/Engine.CharacterMovementComponent|SetBrakingDecelerationWalking _charactermovement 1.0))
      (Variables|/Script/Engine.CharacterMovementComponent|SetBrakingFrictionFactor _charactermovement _output_get_3)
      (if _returnvalue
        (goto _label_2)
        (else
          (goto _label)))))
  ;[1 0.9448 0.3267] Spear Grapple
  (if (Utilities|IsValid (Variables|Default|GetSpearObject))
    (Variables|/Script/Engine.MovementComponent|SetVelocity _charactermovement_2 (+ (* (Math|Vector|GetForwardVector (Variables|Default|GetCamera)) (* (Variables|Default|GetPullStrength) 0.5)) (+ (* (Math|Vector|GetUnitDirection(Vector) (Transformation|GetWorldLocation (Variables|Collision|GetCapsuleComponent)) (Transformation|GetWorldLocation (Variables|/Script/Engine.StaticMeshActor|GetStaticMeshComponent (Variables|Default|GetSpearObject)))) (Variables|Default|GetPullStrength)) (Variables|/Script/Engine.MovementComponent|GetVelocity _charactermovement_2))))))

(event Input|ActionEvents|InputActionJump
  (params (Key :type Key%20Structure :default "None"))
  ;[1 0.9448 0.3267] Jump (Jump Buffer for bunny hopping)
  (:Pressed
    (bind _output_get (Variables|Default|SetJumpBuffer 0.1))))

(event Input|ActionEvents|InputActionSlide
  (params (Key :type Key%20Structure :default "None"))
  (bind _camera (Variables|Default|GetCamera))
  ;[1 0.9448 0.3267] Sliding
  (:Pressed
    (Transformation|SetRelativeLocation _camera "0, 0, 0" false false)
    (Character|Crouch)
    (Variables|Default|SetCrouching true))
  (:Released
    (Transformation|SetRelativeLocation _camera "0, 0,50.000000" false false)
    (Character|UnCrouch)
    (Variables|Default|SetCrouching false)))

(event Input|ActionEvents|InputActionThrowSpear
  (params (Key :type Key%20Structure :default "None"))
  ;[0.227 1 0.1517] Throw Spear
  (:Pressed
    (if (not (Variables|Default|GetSpearThrown))
      (bind _returnvalue (Game|SpawnActorfromClass "/Game/Blueprints/SpearProjectile.SpearProjectile_C" (Transformation|GetWorldTransform (Variables|Default|GetThrowFrom)) "Undefined" 0 0))
      (Variables|Default|SetSpearProjectile _returnvalue)
      (Variables|Default|SetSpearThrown true))))

(event Input|ActionEvents|InputActionReturnSpear
  (params (Key :type Key%20Structure :default "None"))
  (bind _spearobject (Variables|Default|GetSpearObject))
  ;[0.227 1 0.1517] Pull Spear
  (:Pressed
    (if (Variables|Default|GetSpearThrown)
      (if (Utilities|IsValid _spearobject)
        (Actor|DestroyActor _spearobject)
        (else
          (Actor|DestroyActor (Variables|Default|GetSpearProjectile))))
      (Variables|Default|SetSpearThrown false)
      (Class|NiagaraComponent|SetNiagaraVariableVec3 (Variables|Default|GetRope) "EndPosition" "10.000000, 0, 0"))))

(event Input|ActionEvents|InputActionAirStrafeRight
  (params (Key :type Key%20Structure :default "None"))
  (bind _charactermovement (Variables|Character|GetCharacterMovement))
  ;[0.09783 0.1892 1] Air Strafe
  (:Pressed
    (if (not (AI|Components|NavMovement|IsMovingonGround (Variables|Character|GetCharacterMovement)))
      (Variables|/Script/Engine.MovementComponent|SetVelocity _charactermovement (+ (Variables|/Script/Engine.MovementComponent|GetVelocity _charactermovement) (* (Transformation|GetActorRightVector) 1e+02))))))

(event Input|ActionEvents|InputActionAirStrafeLeft
  (params (Key :type Key%20Structure :default "None"))
  (bind _charactermovement (Variables|Character|GetCharacterMovement))
  ;[0.09783 0.1892 1] Air Strafe
  (:Pressed
    (if (not (AI|Components|NavMovement|IsMovingonGround (Variables|Character|GetCharacterMovement)))
      (Variables|/Script/Engine.MovementComponent|SetVelocity _charactermovement (+ (Variables|/Script/Engine.MovementComponent|GetVelocity _charactermovement) (* (Transformation|GetActorRightVector) -1e+02))))))

(event Input|AxisEvents|InputAxisHorizontalMovement
  (params (AxisValue :type Float%20%28single-precision%29))
  ;[0.09783 0.1892 1] Movement
  (if (not (Variables|Default|GetSliding))
    (Pawn|Input|AddMovementInput (Transformation|GetActorRightVector) AxisValue false)))

(event Input|AxisEvents|InputAxisVerticalRotation
  (params (AxisValue :type Float%20%28single-precision%29))
  (bind _camera (Variables|Default|GetCamera))
  ;[0.09783 0.1892 1] Look
  (if (<= (Math|Float|Absolute(Float) (+ AxisValue (.pitch (Transformation|GetWorldRotation _camera)))) 85.0)
    (Transformation|AddLocalRotation _camera (Math|Rotator|MakeRotator 0.0 AxisValue 0.0) false false)))

(event Input|AxisEvents|InputAxisHorizontalRotation
  (params (AxisValue :type Float%20%28single-precision%29))
  ;[0.09783 0.1892 1] Look
  (Pawn|Input|AddControllerYawInput AxisValue))

(event Input|AxisEvents|InputAxisVerticalMovement
  (params (AxisValue :type Float%20%28single-precision%29))
  ;[0.09783 0.1892 1] Movement
  (if (not (Variables|Default|GetSliding))
    (Pawn|Input|AddMovementInput (Transformation|GetActorForwardVector) AxisValue false)))

(fn ConstructionScript)